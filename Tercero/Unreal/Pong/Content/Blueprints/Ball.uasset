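; Bouncing ball actor that moves at constant Speed and scores points for two sides, Pong-style.
; BeginPlay launches the physics sphere at a random yaw off its right vector, rolled separately from the stored CurrentDirection.
; Each hit reflects CurrentDirection off the surface normal, adds slight random yaw jitter and resets velocity.
; Overlapping Impacto1 or Impacto2 increments PlayerScore or PlayerScore2 on MyPlayerController, without resetting the ball.
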(event Collision|EventActorBeginOverlap
  (params (OtherActor :type Actor%20Object%20Reference))
  (bind _controller (Variables|Default|Getcontroller))
  (if (Collision|IsOverlappingActor (Variables|Default|GetImpacto1) :!class /Script/Engine.Actor)
    (bind _result (Math|Integer|IncrementInt (Variables|/Game/Blueprints/CambioDeEscena/MyPlayerController.MyPlayerController_C|GetPlayer%20Score _controller))
      (:%20%20
        (Variables|/Game/Blueprints/CambioDeEscena/MyPlayerController.MyPlayerController_C|SetPlayer%20Score _controller _result)))
    (elif (Collision|IsOverlappingActor (Variables|Default|GetImpacto2) :!class /Script/Engine.Actor)
      (bind _result_2 (Math|Integer|IncrementInt (Variables|/Game/Blueprints/CambioDeEscena/MyPlayerController.MyPlayerController_C|GetPlayer%20Score2 _controller))
        (:%20%20
          (Variables|/Game/Blueprints/CambioDeEscena/MyPlayerController.MyPlayerController_C|SetPlayer%20Score2 _controller _result_2))))))

(event EventTick
  (params (DeltaSeconds :type Float%20%28single-precision%29)))

(event EventBeginPlay
  (bind _returnvalue (Math|Random|RandomFloatinRange 5.0 3e+01))
  (bind _sphere (Variables|Default|GetSphere))
  (bind _returnvalue_2 (Math|Vector|GetRightVector _sphere))
  (bind _returnvalue_3 (Math|Vector|RotateVector _returnvalue_2 (Math|Rotator|MakeRotator 0.0 0.0 _returnvalue)))
  (Variables|Default|SetCurrent%20Direction _returnvalue_3)
  (Physics|SetPhysicsLinearVelocity (Variables|Default|GetSphere) (* _returnvalue_3 (Variables|Default|GetSpeed)) false "None")
  (bind _asmy_player_controller (Utilities|Casting|CastToMyPlayerController (Game|GetPlayerController 0)))
  (Variables|Default|Setcontroller _asmy_player_controller))

(event Collision|EventHit
  (params (MyComp :type Primitive%20Component%20Object%20Reference) (Other :type Actor%20Object%20Reference) (OtherComp :type Primitive%20Component%20Object%20Reference) (bSelfMoved :type Boolean) (HitLocation :type Vector :default "0, 0, 0") (HitNormal :type Vector :default "0, 0, 0") (NormalImpulse :type Vector :default "0, 0, 0") (Hit :type Hit%20Result%20Structure%20%28by%20ref%29))
  (bind _output_get (Variables|Default|SetCurrent%20Direction (Math|Vector|RotateVector (Math|Vector|Normalize (Math|Vector|GetReflectionVector (Variables|Default|GetCurrent%20Direction) HitNormal)) (Math|Rotator|MakeRotator 0.0 0.0 (Math|Random|RandomFloatinRange -5.0 5.0)))))
  (Physics|SetPhysicsLinearVelocity (Variables|Default|GetSphere) (* _output_get (Variables|Default|GetSpeed)) false "None"))

(fn ConstructionScript)