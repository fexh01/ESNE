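; Player controller for a Pong game that handles switching between the start, match and end levels and their UI.
; BeginPlay checks the current level name and adds the matching widget, enabling the mouse cursor only on the start screen.
; Custom events clear widgets and open the start or game level.
; The match-end event saves both players' scores to a save slot before loading the final level.
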(event Custom|Fin%20de%20Partida
  ;[1 1 1] Guarda la información de la partida
  (bind _returnvalue (SaveGame|CreateSaveGameObject "/Game/Blueprints/CambioDeEscena/MySaveGame.MySaveGame_C"))
  (bind _output_get (Variables|Default|SetMyGame _returnvalue))
  (Variables|/Game/Blueprints/CambioDeEscena/MySaveGame.MySaveGame_C|SetPuntuacion _output_get (Variables|Default|GetPlayer%20Score))
  (Variables|/Game/Blueprints/CambioDeEscena/MySaveGame.MySaveGame_C|SetPuntuacion2 _output_get (Variables|Default|GetPlayer%20Score2))
  (SaveGame|SaveGametoSlot (Variables|Default|GetMyGame) "01")
  ;[1 1 1] Carga el nuevo mapa
  (Game|OpenLevel(byName) "Final"))

(event Custom|Jugar
  (Game|OpenLevel(byName) "Pong")
  (Viewport|RemoveAllWidgets))

(event Custom|Inicio
  (Game|OpenLevel(byName) "Inicio")
  (Viewport|RemoveAllWidgets))

(event EventBeginPlay
  ;[1 1 1] Crea UI y muestra el cursor
  (bind _returnvalue (Game|GetCurrentLevelName true))
  (if (Utilities|Enum|Equal(Enum) _returnvalue "Inicio")
    (bind _returnvalue_2 (UserInterface|CreateWidget "/Game/Blueprints/CambioDeEscena/WidgetInicio.WidgetInicio_C" self))
    (UserInterface|Viewport|AddtoViewport _returnvalue_2 0)
    (Variables|Default|SetbShowMouseCursor true)
    (elif (Utilities|Enum|Equal(Enum) _returnvalue "Pong")
      (bind _returnvalue_3 (UserInterface|CreateWidget "/Game/Blueprints/PongWidget.PongWidget_C" self))
      (UserInterface|Viewport|AddtoViewport _returnvalue_3 0)
      (elif (Utilities|Enum|Equal(Enum) _returnvalue "Final")
        (bind _returnvalue_4 (UserInterface|CreateWidget "/Game/Blueprints/CambioDeEscena/WidgetFinal.WidgetFinal_C" self))
        (UserInterface|Viewport|AddtoViewport _returnvalue_4 0)))))

(event EventTick
  (params (DeltaSeconds :type Float%20%28single-precision%29)))

(fn ConstructionScript)